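; Enemy actor that destroys itself on any overlap and updates the player's health or score.
; Contact with the player decrements BP_Player Health, and reaching exactly zero sets IsDead and calls DisplayRestart.
; An overlap with any other actor adds two points to the player's Score, with no check on what that actor is.
; All logic runs in ActorBeginOverlap, and a leftover Count assignment never runs.
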(event EventBeginPlay)

(event EventTick
  (params (DeltaSeconds :type Float%20%28single-precision%29)))

(event Collision|EventActorBeginOverlap
  (params (OtherActor :type Actor%20Object%20Reference))
  (bind _returnvalue (Game|Player|GetPlayerPawn 0))
  (Actor|DestroyActor)
  (if (== OtherActor (Game|Player|GetPlayerPawn 0))
    (bind _asbp_player (Utilities|Casting|CastToBP_Player _returnvalue))
    (bind _result (Math|Float|DecrementFloat (Variables|/Game/InfiniteMatrix/Blueprints/BP_Player.BP_Player_C|GetHealth _asbp_player))
      (:%20%20
        (if (== _result 0.0)
          (Variables|/Game/InfiniteMatrix/Blueprints/BP_Player.BP_Player_C|SetIsDead _asbp_player true)
          (Default|DisplayRestart _asbp_player)
          (bind _asbp_player_2 (Utilities|Casting|CastToBP_Player (Game|Player|GetPlayerPawn 0))))))
    (else
      (bind _asbp_player_3 (Utilities|Casting|CastToBP_Player _returnvalue))
      (Variables|/Game/InfiniteMatrix/Blueprints/BP_Player.BP_Player_C|SetScore _asbp_player_3 (+ (Variables|/Game/InfiniteMatrix/Blueprints/BP_Player.BP_Player_C|GetScore _asbp_player_3) 2)))))

(fn ConstructionScript)